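; Wind particle actor that wanders in 2D through a simulation volume as a Physarum-style agent steered by a shared trail map.
; Each tick it samples the Trailmap render target at a lookahead point, decoding average direction from RG and weight from B.
; It blends that consensus with random jitter, restores target speed and bounces off SimulationBounds.
; The resulting velocity drives ProjectileMovement and the DrawToTrailmap mesh material's Velocity parameter.
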(event EventBeginPlay
  ;[1 1 1] Start with random velocity
  (Game|Components|ProjectileMovement|SetVelocityinLocalSpace (Variables|Default|GetProjectileMovement) (* (Math|Vector|Normalize (Math|Random|RandomPointinBoundingBox "0, 0, 0" "1.000000,1.000000,0.000000")) (Variables|Default|GetTarget%20Speed))))

(event EventTick
  (params (DeltaSeconds :type Float%20%28single-precision%29))
  (bind _returnvalue (Transformation|GetActorLocation))
  (bind _returnvalue_2 (Transformation|GetActorLocation))
  (bind _projectilemovement (Variables|Default|GetProjectileMovement))
  (bind _simulation_bounds (Variables|Default|GetSimulation%20Bounds))
  (bind _projectilemovement_2 (Variables|Default|GetProjectileMovement))
  (bind _steering_lookahead (Variables|Default|GetSteering%20Lookahead))
  (bind _simulation_bounds_2 (Variables|Default|GetSimulation%20Bounds))
  (bind (_origin _boxextent) (Collision|GetActorBounds _simulation_bounds_2 false true))
  (bind (_origin_2 _boxextent_2) (Collision|GetActorBounds _simulation_bounds false true))
  (bind (_x _y) (Math|Vector|BreakVector _returnvalue_2))
  (bind _velocity (Variables|/Script/Engine.MovementComponent|GetVelocity _projectilemovement))
  (bind _velocity_2 (Variables|/Script/Engine.MovementComponent|GetVelocity _projectilemovement_2))
  (bind _returnvalue_3 (Math|Vector|Normalize _velocity_2))
  (bind _returnvalue_4 (- _origin_2 _boxextent_2))
  (bind _returnvalue_5 (- _origin _boxextent))
  (bind _returnvalue_6 (* _boxextent 2.0))
  (bind _returnvalue_7 (+ _origin_2 _boxextent_2))
  (bind _returnvalue_8 (* _returnvalue_3 _steering_lookahead))
  (bind (_x_2 _y_2) (Math|Vector|BreakVector _returnvalue_4))
  (bind (_x_3 _y_3) (Math|Vector|BreakVector _returnvalue_7))
  (bind _returnvalue_9 (+ _returnvalue _returnvalue_8))
  (bind _returnvalue_10 (- _returnvalue_9 _returnvalue_5))
  (bind _returnvalue_11 (/ _returnvalue_10 _returnvalue_6))
  (bind (_x_4 _y_4) (Math|Vector|BreakVector _returnvalue_11))
  (Rendering|Debug|DrawDebugArrow :LineStart _returnvalue :LineEnd _returnvalue_9)
  ;[1 1 1] Sample trailmap and decode vector
  (bind _returnvalue_12 (Class|KismetRenderingLibrary|ReadRenderTargetUV (Variables|Default|GetTrailmap) _x_4 _y_4))
  (Game|Components|ProjectileMovement|SetVelocityinLocalSpace (Variables|Default|GetProjectileMovement) (Math|Vector|MakeVector (select (> _x _x_3) (* -1 (Math|Float|Absolute(Float) (.X (Math|Vector|BreakVector (* (Math|Vector|Normalize (+ (Math|Vector|Normalize _velocity) (* (Math|Vector|Normalize (- (* (/ (Math|Vector|MakeVector (.R (Math|Color|BreakColor (Math|Conversions|ToLinearColor(Color) _returnvalue_12))) (.G (Math|Color|BreakColor (Math|Conversions|ToLinearColor(Color) _returnvalue_12))) 0.0) (.B (Math|Color|BreakColor (Math|Conversions|ToLinearColor(Color) _returnvalue_12)))) 2.0) "1.000000,1.000000, 0")) (* (Math|Float|Sqrt (.B (Math|Color|BreakColor (Math|Conversions|ToLinearColor(Color) _returnvalue_12)))) (Variables|Default|GetSteering%20Force))) (* (Math|Vector|Normalize (Math|Random|RandomPointinBoundingBox "0, 0, 0" "1.000000,1.000000, 0")) (Variables|Default|GetRandom%20Force)))) (Math|Float|Lerp (Math|Vector|VectorLength _velocity) (Variables|Default|GetTarget%20Speed) (Variables|Default|GetSpeed%20Restoration%20Force))))))) (select (< _x _x_2) (Math|Float|Absolute(Float) (.X (Math|Vector|BreakVector (* (Math|Vector|Normalize (+ (Math|Vector|Normalize _velocity) (* (Math|Vector|Normalize (- (* (/ (Math|Vector|MakeVector (.R (Math|Color|BreakColor (Math|Conversions|ToLinearColor(Color) _returnvalue_12))) (.G (Math|Color|BreakColor (Math|Conversions|ToLinearColor(Color) _returnvalue_12))) 0.0) (.B (Math|Color|BreakColor (Math|Conversions|ToLinearColor(Color) _returnvalue_12)))) 2.0) "1.000000,1.000000, 0")) (* (Math|Float|Sqrt (.B (Math|Color|BreakColor (Math|Conversions|ToLinearColor(Color) _returnvalue_12)))) (Variables|Default|GetSteering%20Force))) (* (Math|Vector|Normalize (Math|Random|RandomPointinBoundingBox "0, 0, 0" "1.000000,1.000000, 0")) (Variables|Default|GetRandom%20Force)))) (Math|Float|Lerp (Math|Vector|VectorLength _velocity) (Variables|Default|GetTarget%20Speed) (Variables|Default|GetSpeed%20Restoration%20Force)))))) (.X (Math|Vector|BreakVector (* (Math|Vector|Normalize (+ (Math|Vector|Normalize _velocity) (* (Math|Vector|Normalize (- (* (/ (Math|Vector|MakeVector (.R (Math|Color|BreakColor (Math|Conversions|ToLinearColor(Color) _returnvalue_12))) (.G (Math|Color|BreakColor (Math|Conversions|ToLinearColor(Color) _returnvalue_12))) 0.0) (.B (Math|Color|BreakColor (Math|Conversions|ToLinearColor(Color) _returnvalue_12)))) 2.0) "1.000000,1.000000, 0")) (* (Math|Float|Sqrt (.B (Math|Color|BreakColor (Math|Conversions|ToLinearColor(Color) _returnvalue_12)))) (Variables|Default|GetSteering%20Force))) (* (Math|Vector|Normalize (Math|Random|RandomPointinBoundingBox "0, 0, 0" "1.000000,1.000000, 0")) (Variables|Default|GetRandom%20Force)))) (Math|Float|Lerp (Math|Vector|VectorLength _velocity) (Variables|Default|GetTarget%20Speed) (Variables|Default|GetSpeed%20Restoration%20Force))))))) (select (> _y _y_3) (* -1 (Math|Float|Absolute(Float) (.Y (Math|Vector|BreakVector (* (Math|Vector|Normalize (+ (Math|Vector|Normalize _velocity) (* (Math|Vector|Normalize (- (* (/ (Math|Vector|MakeVector (.R (Math|Color|BreakColor (Math|Conversions|ToLinearColor(Color) _returnvalue_12))) (.G (Math|Color|BreakColor (Math|Conversions|ToLinearColor(Color) _returnvalue_12))) 0.0) (.B (Math|Color|BreakColor (Math|Conversions|ToLinearColor(Color) _returnvalue_12)))) 2.0) "1.000000,1.000000, 0")) (* (Math|Float|Sqrt (.B (Math|Color|BreakColor (Math|Conversions|ToLinearColor(Color) _returnvalue_12)))) (Variables|Default|GetSteering%20Force))) (* (Math|Vector|Normalize (Math|Random|RandomPointinBoundingBox "0, 0, 0" "1.000000,1.000000, 0")) (Variables|Default|GetRandom%20Force)))) (Math|Float|Lerp (Math|Vector|VectorLength _velocity) (Variables|Default|GetTarget%20Speed) (Variables|Default|GetSpeed%20Restoration%20Force))))))) (select (< _y _y_2) (Math|Float|Absolute(Float) (.Y (Math|Vector|BreakVector (* (Math|Vector|Normalize (+ (Math|Vector|Normalize _velocity) (* (Math|Vector|Normalize (- (* (/ (Math|Vector|MakeVector (.R (Math|Color|BreakColor (Math|Conversions|ToLinearColor(Color) _returnvalue_12))) (.G (Math|Color|BreakColor (Math|Conversions|ToLinearColor(Color) _returnvalue_12))) 0.0) (.B (Math|Color|BreakColor (Math|Conversions|ToLinearColor(Color) _returnvalue_12)))) 2.0) "1.000000,1.000000, 0")) (* (Math|Float|Sqrt (.B (Math|Color|BreakColor (Math|Conversions|ToLinearColor(Color) _returnvalue_12)))) (Variables|Default|GetSteering%20Force))) (* (Math|Vector|Normalize (Math|Random|RandomPointinBoundingBox "0, 0, 0" "1.000000,1.000000, 0")) (Variables|Default|GetRandom%20Force)))) (Math|Float|Lerp (Math|Vector|VectorLength _velocity) (Variables|Default|GetTarget%20Speed) (Variables|Default|GetSpeed%20Restoration%20Force)))))) (.Y (Math|Vector|BreakVector (* (Math|Vector|Normalize (+ (Math|Vector|Normalize _velocity) (* (Math|Vector|Normalize (- (* (/ (Math|Vector|MakeVector (.R (Math|Color|BreakColor (Math|Conversions|ToLinearColor(Color) _returnvalue_12))) (.G (Math|Color|BreakColor (Math|Conversions|ToLinearColor(Color) _returnvalue_12))) 0.0) (.B (Math|Color|BreakColor (Math|Conversions|ToLinearColor(Color) _returnvalue_12)))) 2.0) "1.000000,1.000000, 0")) (* (Math|Float|Sqrt (.B (Math|Color|BreakColor (Math|Conversions|ToLinearColor(Color) _returnvalue_12)))) (Variables|Default|GetSteering%20Force))) (* (Math|Vector|Normalize (Math|Random|RandomPointinBoundingBox "0, 0, 0" "1.000000,1.000000, 0")) (Variables|Default|GetRandom%20Force)))) (Math|Float|Lerp (Math|Vector|VectorLength _velocity) (Variables|Default|GetTarget%20Speed) (Variables|Default|GetSpeed%20Restoration%20Force))))))) (.Z (Math|Vector|BreakVector (* (Math|Vector|Normalize (+ (Math|Vector|Normalize _velocity) (* (Math|Vector|Normalize (- (* (/ (Math|Vector|MakeVector (.R (Math|Color|BreakColor (Math|Conversions|ToLinearColor(Color) _returnvalue_12))) (.G (Math|Color|BreakColor (Math|Conversions|ToLinearColor(Color) _returnvalue_12))) 0.0) (.B (Math|Color|BreakColor (Math|Conversions|ToLinearColor(Color) _returnvalue_12)))) 2.0) "1.000000,1.000000, 0")) (* (Math|Float|Sqrt (.B (Math|Color|BreakColor (Math|Conversions|ToLinearColor(Color) _returnvalue_12)))) (Variables|Default|GetSteering%20Force))) (* (Math|Vector|Normalize (Math|Random|RandomPointinBoundingBox "0, 0, 0" "1.000000,1.000000, 0")) (Variables|Default|GetRandom%20Force)))) (Math|Float|Lerp (Math|Vector|VectorLength _velocity) (Variables|Default|GetTarget%20Speed) (Variables|Default|GetSpeed%20Restoration%20Force)))))))
  ;[1 1 1] Update color to represent velocity
  (bind _asstatic_mesh_component (Utilities|Casting|CastToStaticMeshComponent (Components|GetChildComponent (Variables|Default|GetDrawToTrailmap) 0)))
  (bind _asmaterial_instance_dynamic (Utilities|Casting|CastToMaterialInstanceDynamic (Rendering|Material|GetMaterial _asstatic_mesh_component 0)))
  (Rendering|Material|SetVectorParameterValue _asmaterial_instance_dynamic "Velocity" (Math|Conversions|ToLinearColor(Vector) (Math|Vector|MakeVector (select (> _x _x_3) (* -1 (Math|Float|Absolute(Float) (.X (Math|Vector|BreakVector (* (Math|Vector|Normalize (+ (Math|Vector|Normalize _velocity) (* (Math|Vector|Normalize (- (* (/ (Math|Vector|MakeVector (.R (Math|Color|BreakColor (Math|Conversions|ToLinearColor(Color) _returnvalue_12))) (.G (Math|Color|BreakColor (Math|Conversions|ToLinearColor(Color) _returnvalue_12))) 0.0) (.B (Math|Color|BreakColor (Math|Conversions|ToLinearColor(Color) _returnvalue_12)))) 2.0) "1.000000,1.000000, 0")) (* (Math|Float|Sqrt (.B (Math|Color|BreakColor (Math|Conversions|ToLinearColor(Color) _returnvalue_12)))) (Variables|Default|GetSteering%20Force))) (* (Math|Vector|Normalize (Math|Random|RandomPointinBoundingBox "0, 0, 0" "1.000000,1.000000, 0")) (Variables|Default|GetRandom%20Force)))) (Math|Float|Lerp (Math|Vector|VectorLength _velocity) (Variables|Default|GetTarget%20Speed) (Variables|Default|GetSpeed%20Restoration%20Force))))))) (select (< _x _x_2) (Math|Float|Absolute(Float) (.X (Math|Vector|BreakVector (* (Math|Vector|Normalize (+ (Math|Vector|Normalize _velocity) (* (Math|Vector|Normalize (- (* (/ (Math|Vector|MakeVector (.R (Math|Color|BreakColor (Math|Conversions|ToLinearColor(Color) _returnvalue_12))) (.G (Math|Color|BreakColor (Math|Conversions|ToLinearColor(Color) _returnvalue_12))) 0.0) (.B (Math|Color|BreakColor (Math|Conversions|ToLinearColor(Color) _returnvalue_12)))) 2.0) "1.000000,1.000000, 0")) (* (Math|Float|Sqrt (.B (Math|Color|BreakColor (Math|Conversions|ToLinearColor(Color) _returnvalue_12)))) (Variables|Default|GetSteering%20Force))) (* (Math|Vector|Normalize (Math|Random|RandomPointinBoundingBox "0, 0, 0" "1.000000,1.000000, 0")) (Variables|Default|GetRandom%20Force)))) (Math|Float|Lerp (Math|Vector|VectorLength _velocity) (Variables|Default|GetTarget%20Speed) (Variables|Default|GetSpeed%20Restoration%20Force)))))) (.X (Math|Vector|BreakVector (* (Math|Vector|Normalize (+ (Math|Vector|Normalize _velocity) (* (Math|Vector|Normalize (- (* (/ (Math|Vector|MakeVector (.R (Math|Color|BreakColor (Math|Conversions|ToLinearColor(Color) _returnvalue_12))) (.G (Math|Color|BreakColor (Math|Conversions|ToLinearColor(Color) _returnvalue_12))) 0.0) (.B (Math|Color|BreakColor (Math|Conversions|ToLinearColor(Color) _returnvalue_12)))) 2.0) "1.000000,1.000000, 0")) (* (Math|Float|Sqrt (.B (Math|Color|BreakColor (Math|Conversions|ToLinearColor(Color) _returnvalue_12)))) (Variables|Default|GetSteering%20Force))) (* (Math|Vector|Normalize (Math|Random|RandomPointinBoundingBox "0, 0, 0" "1.000000,1.000000, 0")) (Variables|Default|GetRandom%20Force)))) (Math|Float|Lerp (Math|Vector|VectorLength _velocity) (Variables|Default|GetTarget%20Speed) (Variables|Default|GetSpeed%20Restoration%20Force))))))) (select (> _y _y_3) (* -1 (Math|Float|Absolute(Float) (.Y (Math|Vector|BreakVector (* (Math|Vector|Normalize (+ (Math|Vector|Normalize _velocity) (* (Math|Vector|Normalize (- (* (/ (Math|Vector|MakeVector (.R (Math|Color|BreakColor (Math|Conversions|ToLinearColor(Color) _returnvalue_12))) (.G (Math|Color|BreakColor (Math|Conversions|ToLinearColor(Color) _returnvalue_12))) 0.0) (.B (Math|Color|BreakColor (Math|Conversions|ToLinearColor(Color) _returnvalue_12)))) 2.0) "1.000000,1.000000, 0")) (* (Math|Float|Sqrt (.B (Math|Color|BreakColor (Math|Conversions|ToLinearColor(Color) _returnvalue_12)))) (Variables|Default|GetSteering%20Force))) (* (Math|Vector|Normalize (Math|Random|RandomPointinBoundingBox "0, 0, 0" "1.000000,1.000000, 0")) (Variables|Default|GetRandom%20Force)))) (Math|Float|Lerp (Math|Vector|VectorLength _velocity) (Variables|Default|GetTarget%20Speed) (Variables|Default|GetSpeed%20Restoration%20Force))))))) (select (< _y _y_2) (Math|Float|Absolute(Float) (.Y (Math|Vector|BreakVector (* (Math|Vector|Normalize (+ (Math|Vector|Normalize _velocity) (* (Math|Vector|Normalize (- (* (/ (Math|Vector|MakeVector (.R (Math|Color|BreakColor (Math|Conversions|ToLinearColor(Color) _returnvalue_12))) (.G (Math|Color|BreakColor (Math|Conversions|ToLinearColor(Color) _returnvalue_12))) 0.0) (.B (Math|Color|BreakColor (Math|Conversions|ToLinearColor(Color) _returnvalue_12)))) 2.0) "1.000000,1.000000, 0")) (* (Math|Float|Sqrt (.B (Math|Color|BreakColor (Math|Conversions|ToLinearColor(Color) _returnvalue_12)))) (Variables|Default|GetSteering%20Force))) (* (Math|Vector|Normalize (Math|Random|RandomPointinBoundingBox "0, 0, 0" "1.000000,1.000000, 0")) (Variables|Default|GetRandom%20Force)))) (Math|Float|Lerp (Math|Vector|VectorLength _velocity) (Variables|Default|GetTarget%20Speed) (Variables|Default|GetSpeed%20Restoration%20Force)))))) (.Y (Math|Vector|BreakVector (* (Math|Vector|Normalize (+ (Math|Vector|Normalize _velocity) (* (Math|Vector|Normalize (- (* (/ (Math|Vector|MakeVector (.R (Math|Color|BreakColor (Math|Conversions|ToLinearColor(Color) _returnvalue_12))) (.G (Math|Color|BreakColor (Math|Conversions|ToLinearColor(Color) _returnvalue_12))) 0.0) (.B (Math|Color|BreakColor (Math|Conversions|ToLinearColor(Color) _returnvalue_12)))) 2.0) "1.000000,1.000000, 0")) (* (Math|Float|Sqrt (.B (Math|Color|BreakColor (Math|Conversions|ToLinearColor(Color) _returnvalue_12)))) (Variables|Default|GetSteering%20Force))) (* (Math|Vector|Normalize (Math|Random|RandomPointinBoundingBox "0, 0, 0" "1.000000,1.000000, 0")) (Variables|Default|GetRandom%20Force)))) (Math|Float|Lerp (Math|Vector|VectorLength _velocity) (Variables|Default|GetTarget%20Speed) (Variables|Default|GetSpeed%20Restoration%20Force))))))) (.Z (Math|Vector|BreakVector (* (Math|Vector|Normalize (+ (Math|Vector|Normalize _velocity) (* (Math|Vector|Normalize (- (* (/ (Math|Vector|MakeVector (.R (Math|Color|BreakColor (Math|Conversions|ToLinearColor(Color) _returnvalue_12))) (.G (Math|Color|BreakColor (Math|Conversions|ToLinearColor(Color) _returnvalue_12))) 0.0) (.B (Math|Color|BreakColor (Math|Conversions|ToLinearColor(Color) _returnvalue_12)))) 2.0) "1.000000,1.000000, 0")) (* (Math|Float|Sqrt (.B (Math|Color|BreakColor (Math|Conversions|ToLinearColor(Color) _returnvalue_12)))) (Variables|Default|GetSteering%20Force))) (* (Math|Vector|Normalize (Math|Random|RandomPointinBoundingBox "0, 0, 0" "1.000000,1.000000, 0")) (Variables|Default|GetRandom%20Force)))) (Math|Float|Lerp (Math|Vector|VectorLength _velocity) (Variables|Default|GetTarget%20Speed) (Variables|Default|GetSpeed%20Restoration%20Force))))))) :!class /Script/Engine.MaterialInstanceDynamic))

(fn ConstructionScript)