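; Wind system manager that simulates wind with particle actors and render targets, and spawns wisps that follow it.
; BeginPlay scatters BP_WindParticle actors in SpawnBox and clears the trailmap.
; Tick ping-pongs the trailmap through a back buffer and rebuilds avoidance gradients from terrain and scene into a final target.
; A randomized, re-arming timer spawns BP_WindWisp at a set height, oriented by a direction decoded from trailmap pixels.
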(event Custom|Spawn%20Wisp
  (bind _spawn_box (Variables|Default|GetSpawn%20Box))
  (bind (_origin _boxextent) (Collision|GetActorBounds _spawn_box false false))
  (bind _returnvalue (Math|Random|RandomPointinBoundingBox _origin _boxextent))
  (bind _returnvalue_2 (- _origin _boxextent))
  (bind _returnvalue_3 (- _returnvalue _returnvalue_2))
  (bind (_x _y) (Math|Vector|BreakVector _returnvalue))
  (bind _returnvalue_4 (/ _returnvalue_3 _boxextent))
  (bind (_x_2 _y_2) (Math|Vector|BreakVector _returnvalue_4))
  ;[1 1 1] Spawn Wisp on repeat
  (bind _returnvalue_5 (Class|KismetRenderingLibrary|ReadRenderTargetUV "/Game/WindSystem/RT_WindTrailmap.RT_WindTrailmap" _x_2 _y_2))
  (Game|SpawnActorfromClass "/Game/WindSystem/Wisps/BP_WindWisp.BP_WindWisp_C" (Math|Transform|MakeTransform (Math|Vector|MakeVector _x _y (Variables|Default|GetWisp%20Spawn%20Height)) (Math|Rotator|FindLookatRotation (Math|Vector|MakeVector 0.0 0.0 0.0) (+ (* (/ (Math|Vector|MakeVector (.R (Math|Color|BreakColor (Math|Conversions|ToLinearColor(Color) _returnvalue_5))) (.G (Math|Color|BreakColor (Math|Conversions|ToLinearColor(Color) _returnvalue_5))) 0.0) (.B (Math|Color|BreakColor (Math|Conversions|ToLinearColor(Color) _returnvalue_5)))) 2.0) "-1.000000,-1.000000, 0"))) "Undefined" 0 0)
  (Utilities|Time|SetTimerbyEvent (delegate Custom|Spawn%20Wisp) (Math|Random|RandomFloatinRange (Variables|Default|GetWisp%20Spawn%20Rate%20Min) (Variables|Default|GetWisp%20Spawn%20Rate%20Max))))

(event EventBeginPlay
  (bind _returnvalue (Math|Color|MakeColor 0.0 0.0 0.0 0.0))
  (bind _spawn_box (Variables|Default|GetSpawn%20Box))
  (bind (_origin _boxextent) (Collision|GetActorBounds _spawn_box false false))
  (bind (_x _y) (Math|Vector|BreakVector _boxextent))
  ;[1 1 1] Spawn from blueprint within volume
  (for _index (range 1 (Variables|Default|GetSpawn%20Count))
    (bind _returnvalue_2 (Game|SpawnActorfromClass "/Game/WindParticleActor/BP_WindParticle.BP_WindParticle_C" (Math|Transform|MakeTransform (Math|Random|RandomPointinBoundingBox _origin (Math|Vector|MakeVector _x _y 0.0))) "Undefined" 0 0))
    ;[1 1 1] Assign scene references
    (Variables|/Game/WindParticleActor/BP_WindParticle.BP_WindParticle_C|SetSimulation%20Bounds _returnvalue_2 (Variables|Default|GetSpawn%20Box)))
  (Rendering|ClearRenderTarget2D "/Game/WindSystem/RT_WindTrailmap.RT_WindTrailmap" _returnvalue)
  (Rendering|ClearRenderTarget2D "/Game/WindSystem/RT_WindTrailmap_BackBuffer.RT_WindTrailmap_BackBuffer" _returnvalue)
  (bind _returnvalue_3 (Rendering|Material|CreateDynamicMaterialInstance (Variables|Default|GetTrailmap%20Ticker) "None" "None" :!class /Script/Engine.KismetMaterialLibrary))
  ;[1 1 1] Spawn Wisp on repeat
  (Utilities|Time|SetTimerbyEvent (delegate Custom|Spawn%20Wisp) (Math|Random|RandomFloatinRange (Variables|Default|GetWisp%20Spawn%20Rate%20Min) (Variables|Default|GetWisp%20Spawn%20Rate%20Max))))

(event EventTick
  (params (DeltaSeconds :type Float%20%28single-precision%29))
  (Utilities|FlowControl|Sequence
    (:then_0
      ;[1 1 1] Trailmap RT-to-RT pipeline
      (Rendering|DrawMaterialtoRenderTarget "/Game/WindSystem/RT_WindTrailmap_BackBuffer.RT_WindTrailmap_BackBuffer" "/Game/MI_PreviewTrailmapMain.MI_PreviewTrailmapMain")
      (Rendering|DrawMaterialtoRenderTarget "/Game/WindSystem/RT_WindTrailmap.RT_WindTrailmap" (stale EventBeginPlay _returnvalue_3)))
    (:then_1
      (Rendering|DrawMaterialtoRenderTarget "/Game/WindSystem/Collision/RT_WindAvoidRawFromTerrain.RT_WindAvoidRawFromTerrain" "/Game/WindSystem/Collision/MI_TerrainHeightmapToWindCollidable.MI_TerrainHeightmapToWindCollidable")
      (Rendering|DrawMaterialtoRenderTarget "/Game/WindSystem/Collision/RT_WindAvoidGradientFromTerrain.RT_WindAvoidGradientFromTerrain" "/Game/WindSystem/Collision/MI_WindAvoidTerrainRawToGradient.MI_WindAvoidTerrainRawToGradient")
      (Rendering|DrawMaterialtoRenderTarget "/Game/WindSystem/Collision/RT_WindAvoidGradientFromScene.RT_WindAvoidGradientFromScene" "/Game/WindSystem/Collision/MI_WindAvoidSceneRawToGradient.MI_WindAvoidSceneRawToGradient")
      (Rendering|DrawMaterialtoRenderTarget "/Game/WindSystem/Collision/RT_WindAvoidGradientFinal.RT_WindAvoidGradientFinal" "/Game/WindSystem/Collision/M_AvoidBuildFinalGradient.M_AvoidBuildFinalGradient"))))

(fn ConstructionScript)