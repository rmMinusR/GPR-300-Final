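; BP_TrailmapDrawStamp is a wind system actor whose mesh stamps movement direction for a trail map, apparently into a Runtime Virtual Texture.
; On BeginPlay it puts a dynamic instance of M_StampToRVTActor on its static mesh.
; Each tick, when its speed exceeds MinSpeed, it writes the normalized velocity to the material's Velocity parameter.
; At lower speeds the last written direction stays in place.
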(event EventBeginPlay
  (bind _returnvalue (Rendering|Material|CreateDynamicMaterialInstance (Variables|Debug|GetStaticMeshComponent) 0 "/Game/WindSystem/WindParticleActor/M_StampToRVTActor.M_StampToRVTActor" "None" :!class /Script/Engine.PrimitiveComponent))
  (Rendering|Material|SetMaterial (Variables|Debug|GetStaticMeshComponent) 0 _returnvalue))

(event EventTick
  (params (DeltaSeconds :type Float%20%28single-precision%29))
  (bind _returnvalue (Transformation|GetVelocity))
  (if (> (Math|Vector|VectorLength _returnvalue) (Variables|Default|GetMinSpeed))
    (Rendering|Material|SetVectorParameterValue (stale EventBeginPlay _returnvalue) "Velocity" (Math|Conversions|ToLinearColor(Vector) (Math|Vector|Normalize _returnvalue)) :!class /Script/Engine.MaterialInstanceDynamic)))

(fn ConstructionScript)